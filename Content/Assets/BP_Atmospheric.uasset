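; Underwater atmosphere actor that exposes controls for light refraction caustics and marine snow.
; Refraction speed and amount setters write to the MC_WaterParams parameter collection, with amount converted from a percentage.
; The snow quantity setter drives the Count parameter on the MarineSnow effect.
; A run-once event can make the LightRefraction light function material dynamic, but its only callers are unreachable leftover nodes.
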(event Custom|Set%20Refraction%20Speed
  (params (New%20Speed :type Float%20%28single-precision%29))
  (Rendering|Material|SetScalarParameterValue "/Game/Assets/Materials/MC_WaterParams.MC_WaterParams" "Caustics Speed" New%20Speed :!class /Script/Engine.KismetMaterialLibrary))

(event Custom|Set%20Snow%20Quantity
  (params (New%20Quantity :type Float%20%28single-precision%29))
  (Effects|Components|ParticleSystem|SetFloatParameter (Variables|Default|GetMarineSnow) "Count" New%20Quantity))

(event Custom|Set%20Refraction%20Amount
  (params (New%20Percentage :type Float%20%28single-precision%29))
  (Rendering|Material|SetScalarParameterValue "/Game/Assets/Materials/MC_WaterParams.MC_WaterParams" "Caustics Ammount" (* New%20Percentage 0.01) :!class /Script/Engine.KismetMaterialLibrary))

(event Custom|Make%20Refraction%20Dynamic
  (bind _lightrefraction (Variables|Default|GetLightRefraction))
  (Utilities|FlowControl|DoOnce false
    (:Completed
      (bind _returnvalue (Rendering|Material|CreateDynamicMaterialInstance (Variables|/Script/Engine.LightComponent|GetLightFunctionMaterial _lightrefraction) "None" "None" :!class /Script/Engine.KismetMaterialLibrary))
      (bind _output_get (Variables|Default|SetRefractionMaterial _returnvalue))
      (Rendering|Components|Light|SetLightFunctionMaterial _lightrefraction _output_get))))

(fn ConstructionScript)