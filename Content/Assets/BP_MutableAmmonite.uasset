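; Actor that displays a procedurally generated ammonite shell, a ghost shell and a placeholder soft body.
; Tick watches the game state's two shell generators, then bakes finished results, passed through a PNG-based distortion step, into static meshes, with optional low resolution.
; Shell updates rescale to a target radius, fit the soft body to the aperture and rotate by visible whorls.
; Events control orientation, visibility and section-color parameters on dynamic materials.
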(event Custom|Set%20Shell%20Mesh
  (params (Shell%20Mesh :type Static%20Mesh%20Object%20Reference) (Info%20at%20Final%20Theta :type Radius%20Info%20Structure))
  (bind _currentgamestate (Variables|Default|GetCurrentGameState))
  (bind _softbodytemp (Variables|Default|GetSoftbodyTEMP))
  (bind _relativelocation (Variables|/Script/Engine.SceneComponent|GetRelativeLocation _softbodytemp))
  (bind (_x _y _z) (Math|Vector|BreakVector _relativelocation))
  (Variables|Default|SetApertureStats Info%20at%20Final%20Theta)
  (Components|StaticMesh|SetStaticMesh (Variables|Default|GetShell) Shell%20Mesh)
  (CallFunction|RecalculateShellBounds)
  (if (!= (/ (Variables|/Script/Engine.SphereComponent|GetSphereRadius (Variables|Default|GetTargetRadius)) (* (+ (.spiral_radius (Utilities|Struct|BreakRadiusInfo (Variables|Default|GetApertureStats))) (.tube_normal_radius (Utilities|Struct|BreakRadiusInfo (Variables|Default|GetApertureStats)))) 3e+01)) 0.0)
    (Utilities|FlowControl|Sequence
      (:then_0
        (Transformation|SetRelativeScale3D (Variables|Default|GetShellTiltParent) (Math|Vector|MakeVector (/ (Variables|/Script/Engine.SphereComponent|GetSphereRadius (Variables|Default|GetTargetRadius)) (* (+ (.spiral_radius (Utilities|Struct|BreakRadiusInfo (Variables|Default|GetApertureStats))) (.tube_normal_radius (Utilities|Struct|BreakRadiusInfo (Variables|Default|GetApertureStats)))) 3e+01)) (/ (Variables|/Script/Engine.SphereComponent|GetSphereRadius (Variables|Default|GetTargetRadius)) (* (+ (.spiral_radius (Utilities|Struct|BreakRadiusInfo (Variables|Default|GetApertureStats))) (.tube_normal_radius (Utilities|Struct|BreakRadiusInfo (Variables|Default|GetApertureStats)))) 3e+01)) (/ (Variables|/Script/Engine.SphereComponent|GetSphereRadius (Variables|Default|GetTargetRadius)) (* (+ (.spiral_radius (Utilities|Struct|BreakRadiusInfo (Variables|Default|GetApertureStats))) (.tube_normal_radius (Utilities|Struct|BreakRadiusInfo (Variables|Default|GetApertureStats)))) 3e+01)))))
      (:then_1
        (Utilities|FlowControl|Sequence
          (:then_0
            (Transformation|SetRelativeLocation _softbodytemp (Math|Vector|MakeVector (* (.spiral_radius (Utilities|Struct|BreakRadiusInfo (Variables|Default|GetApertureStats))) -3e+01) _y _z) false false))
          (:then_1
            (Transformation|SetRelativeScale3D (Variables|Default|GetSoftbodyTEMP) (* (Math|Vector|MakeVector (.tube_normal_radius (Utilities|Struct|BreakRadiusInfo (Variables|Default|GetApertureStats))) (.tube_binormal_radius (Utilities|Struct|BreakRadiusInfo (Variables|Default|GetApertureStats))) (.tube_normal_radius (Utilities|Struct|BreakRadiusInfo (Variables|Default|GetApertureStats)))) 12.0)))
          (:then_2
            (CallFunction|RotateShellAccordingtoWhorls (* (* (Variables|/Game/System/AmmoniteState.AmmoniteState_C|GetwhorlsPercentVisible _currentgamestate) 0.01) (Variables|/Game/System/AmmoniteState.AmmoniteState_C|GetwhorlsTotal _currentgamestate)))))))))

(event Custom|Set%20Shell%20Material%20Settings
  (params (Show%20Colors :type Boolean) (Section1%20End :type Float%20%28single-precision%29) (Section2%20Start :type Float%20%28single-precision%29) (Section2%20End :type Float%20%28single-precision%29) (Section3%20Start :type Float%20%28single-precision%29) (Section%202%20Enabled :type Boolean) (Section%203%20Enabled :type Boolean))
  (bind _shellmaterial (Variables|Default|GetShellMaterial))
  (if Show%20Colors
    (Utilities|FlowControl|Sequence
      (:then_0
        (Rendering|Material|SetScalarParameterValue _shellmaterial "Show Section Colors" (Math|Conversions|ToFloat(Boolean) Show%20Colors) :!class /Script/Engine.MaterialInstanceDynamic :!label _label))
      (:then_1
        (Rendering|Material|SetScalarParameterValue _shellmaterial "Young Pure End" Section1%20End :!class /Script/Engine.MaterialInstanceDynamic)
        (Rendering|Material|SetScalarParameterValue _shellmaterial "Old Pure Start" Section2%20Start :!class /Script/Engine.MaterialInstanceDynamic)
        (Rendering|Material|SetScalarParameterValue _shellmaterial "Old Pure End" Section2%20End :!class /Script/Engine.MaterialInstanceDynamic)
        (Rendering|Material|SetScalarParameterValue _shellmaterial "Aperture Pure Start" Section3%20Start :!class /Script/Engine.MaterialInstanceDynamic))
      (:then_2
        (Rendering|Material|SetScalarParameterValue _shellmaterial "Section 2 Enabled" (Math|Conversions|ToFloat(Boolean) Section%202%20Enabled) :!class /Script/Engine.MaterialInstanceDynamic)
        (Rendering|Material|SetScalarParameterValue _shellmaterial "Section 3 Enabled" (Math|Conversions|ToFloat(Boolean) Section%203%20Enabled) :!class /Script/Engine.MaterialInstanceDynamic)))
    (else
      (goto _label))))

(event Custom|Allow%20Static%20Mesh%20Update
  (params (Low%20Res%20Generation :type Boolean))
  (Utilities|FlowControl|DoOnce false) ; enters at Reset
)

(event Custom|Set%20Shell%20Roll
  (params (New%20Angle :type Float%20%28single-precision%29))
  (bind _returnvalue (Math|Float|MakeLiteralFloat 9e+01))
  (bind _returnvalue_2 (Math|Float|MakeLiteralFloat -9e+01))
  (bind _defaultsceneroot (Variables|Default|GetDefaultSceneRoot))
  (bind _defaultsceneroot_2 (Variables|Default|GetDefaultSceneRoot))
  (bind _relativerotation (Variables|/Script/Engine.SceneComponent|GetRelativeRotation _defaultsceneroot_2))
  (bind _relativerotation_2 (Variables|/Script/Engine.SceneComponent|GetRelativeRotation _defaultsceneroot))
  (bind _roll (Math|Rotator|BreakRotator _relativerotation))
  (bind (_roll_2 _pitch _yaw) (Math|Rotator|BreakRotator _relativerotation_2))
  (bind _returnvalue_3 (< _roll _returnvalue_2))
  (Transformation|AddRelativeRotation _defaultsceneroot_2 (Math|Rotator|MakeRotator New%20Angle 0.0 0.0) false false)
  (if (or (> _roll _returnvalue) _returnvalue_3)
    (Transformation|SetRelativeRotation _defaultsceneroot (Math|Rotator|MakeRotator (Math|Float|SelectFloat _returnvalue_2 _returnvalue _returnvalue_3) _pitch _yaw) false false)))

(event Custom|Set%20Shell%20Angle
  (params (New%20Angle :type Float%20%28single-precision%29))
  (Transformation|SetRelativeRotation (Variables|Default|GetShellTiltParent) (Math|Rotator|CombineRotators (Math|Rotator|MakeRotator -9e+01 New%20Angle 0.0) "-1.000000,1.000000,0.000000") false false)
  (Transformation|SetRelativeRotation (Variables|Default|GetSoftbodyTEMP) (Math|Rotator|MakeRotator -9e+01 0.0 (- 1.8e+02 New%20Angle)) false false))

(event Custom|Recalculate%20Shell%20Bounds
  (bind _boundspreview (Variables|Default|GetBoundsPreview))
  (bind _shelltiltparent (Variables|Default|GetShellTiltParent))
  (bind _shell (Variables|Default|GetShell))
  (bind (_origin _boxextent _sphereradius) (Collision|GetComponentBounds _shell))
  (bind (_min _max) (Components|StaticMesh|GetLocalBounds _shell))
  (bind _relativescale3d (Variables|/Script/Engine.SceneComponent|GetRelativeScale3D _shell))
  (bind _relativescale3d_2 (Variables|/Script/Engine.SceneComponent|GetRelativeScale3D _shelltiltparent))
  (bind _returnvalue (- _min _max))
  (bind _x (Math|Vector|BreakVector _relativescale3d_2))
  (bind _returnvalue_2 (* _returnvalue 0.5))
  (bind _returnvalue_3 (* _relativescale3d _returnvalue_2))
  (Transformation|SetWorldLocation _boundspreview _origin false false)
  (if (and (Class|KismetMathLibrary|NotEqualExactlyVectorVector _returnvalue_3 "0, 0, 0") (!= _x 0.0))
    (Utilities|FlowControl|Sequence
      (:then_0
        (Components|Box|SetBoxExtent _boundspreview _returnvalue_3 false))
      (:then_1
        (Components|Sphere|SetSphereRadius (Variables|Default|GetRadiusPreview) (/ _sphereradius _x) false)))))

(event Custom|Rotate%20Shell%20About%20Z
  (params (Relative%20Angle :type Float%20%28single-precision%29))
  (Transformation|AddRelativeRotation (Variables|Default|GetDefaultSceneRoot) (Math|Rotator|MakeRotator 0.0 0.0 Relative%20Angle) false false))

(event Custom|Rotate%20Shell%20According%20to%20Whorls
  (params (Number%20of%20180°s :type Float%20%28single-precision%29))
  (Transformation|SetRelativeRotation (Variables|Default|GetShell) (Math|Rotator|MakeRotator 0.0 0.0 (* (- Number%20of%20180°s 1.0) 1.8e+02)) false false))

(event Custom|Set%20Ghost%20Mesh
  (params (New%20Mesh :type Static%20Mesh%20Object%20Reference) (Info%20at%20Final%20Theta :type Radius%20Info%20Structure))
  (bind _currentgamestate (Variables|Default|GetCurrentGameState))
  (Variables|Default|SetApertureStatsGhost Info%20at%20Final%20Theta)
  (Components|StaticMesh|SetStaticMesh (Variables|Default|GetShellGhost) New%20Mesh)
  (Rendering|Material|SetScalarParameterValue (Variables|Default|GetShellGhostMaterial) "Cutoff" (* (Variables|/Game/System/AmmoniteState.AmmoniteState_C|GetwhorlsTotal _currentgamestate) (* (Variables|/Game/System/AmmoniteState.AmmoniteState_C|GetwhorlsPercentVisible _currentgamestate) 0.01)) :!class /Script/Engine.MaterialInstanceDynamic))

(event Custom|Set%20Ghost%20Mesh%20Visibility
  (params (New%20Visibility :type Boolean))
  (Rendering|SetVisibility (Variables|Default|GetShellGhost) New%20Visibility false))

(event Custom|Set%20Softbody%20Visibility
  (params (New%20Visibility :type Boolean))
  (Rendering|SetVisibility (Variables|Default|GetSoftbodyTEMP) New%20Visibility false))

(event Custom|Stats%20Updated
  (Utilities|FlowControl|Sequence
    (:then_0
      _)
    (:then_1
      _))
  (bind _isa (Utilities|FlowControl|FlipFlop)
    (:A
      (CallFunction|AllowStaticMeshUpdate _isa :!label _label))
    (:B
      (Utilities|FlowControl|RetriggerableDelay (Variables|Default|GetupdateRate))
      (if (Variables|Default|GetuseLowResolution)
        (goto _label)))))

(event EventTick
  (params (DeltaSeconds :type Float%20%28single-precision%29))
  (bind _currentgamestate (Variables|Default|GetCurrentGameState))
  (Utilities|FlowControl|Sequence
    (:then_0
      (bind _returnvalue (Class|ShellGenerator|IsGenerationStillinProgress (Variables|/Game/System/AmmoniteState.AmmoniteState_C|GetprimaryShellGenerator _currentgamestate)))
      (bind _returnvalue_2 (Class|ShellGenerator|IsGenerationStillinProgress (Variables|/Game/System/AmmoniteState.AmmoniteState_C|GetghostShellGenerator _currentgamestate)))
      (if (or _returnvalue_2 _returnvalue)
        (goto _label Reset)
        (else
          (Utilities|FlowControl|DoOnce false :!label _label
            (:Completed
              (Utilities|FlowControl|Sequence
                (:then_0
                  _)
                (:then_1
                  _))
              (bind _isa (Utilities|FlowControl|FlipFlop)
                (:A
                  _)
                (:B
                  _))
              (bind (_radius_info _baked_mesh) (Default|GetShell (Variables|Default|GetCurrentGameState) (select (and (stale Custom|Allow%20Static%20Mesh%20Update Low%20Res%20Generation) (Variables|Default|GetuseLowResolution)) (select _isa "NewEnumerator1" "NewEnumerator3") (select _isa "NewEnumerator0" "NewEnumerator2"))))
              (bind _distortions (Utilities|GetOrnament))
              (bind _returnvalue_3 (Class|Distorter|ApplyDistortions _baked_mesh _distortions))
              (bind _returnvalue_4 (Class|MakeStaticMeshLib|BakedMeshtoStaticMesh _returnvalue_3))
              (if _isa
                (CallFunction|SetShellMesh _returnvalue_4 (Utilities|Array|Get(acopy) _radius_info))
                (else
                  (CallFunction|SetGhostMesh _returnvalue_4 (Utilities|Array|Get(acopy) _radius_info)))))))))))

(event EventBeginPlay
  (bind _returnvalue (Game|GetGameState))
  (Utilities|IsValid _returnvalue
    (:Is%20Valid
      (bind _asammonite_state (Utilities|Casting|CastToAmmoniteState _returnvalue))
      (Variables|Default|SetCurrentGameState _asammonite_state)
      (CallFunction|StatsUpdated))
    (:Is%20Not%20Valid
      (Development|PrintString "INVALID GAME STATE REFERENCE ON THE SHELL" true true "(R=1.000000,G=0.004875,B=0.000000,A=1.000000)"))))

(fn ConstructionScript
  (Utilities|FlowControl|Sequence
    (:then_0
      (bind _returnvalue (Class|ShellGenerator|MakeShellGenerator))
      (Variables|Default|SetMainShellGenerator _returnvalue)
      (bind _returnvalue_2 (Class|ShellGenerator|MakeShellGenerator))
      (Variables|Default|SetGhostShellGenerator _returnvalue_2))
    (:then_1
      (CallFunction|RecalculateShellBounds)
      (bind _returnvalue_3 (Rendering|Material|CreateDynamicMaterialInstance (Variables|Default|GetShell) 0 "/Game/Assets/Materials/M_AmmoniteShell.M_AmmoniteShell" "None" :!class /Script/Engine.PrimitiveComponent))
      (Variables|Default|SetShellMaterial _returnvalue_3)
      (bind _returnvalue_4 (Rendering|Material|CreateDynamicMaterialInstance (Variables|Default|GetShellGhost) 0 "/Game/Assets/Materials/M_AmmoniteShellGhost.M_AmmoniteShellGhost" "None" :!class /Script/Engine.PrimitiveComponent))
      (Variables|Default|SetShellGhostMaterial _returnvalue_4))))

(fn GetInfoArrayThetas
  (bind (_initial_expansion _initial_inflation _initial_distance _section_1 _section_2 _section_3 _s1_end _s2_start _s2_end _s3_start _s2_enabled _s3_enabled _total_whorls _whorls_percent_visible) (Default|GetShellStats (Variables|Default|GetCurrentGameState)))
  (Utilities|Array|Clear (LocalVariables|GetThetas))
  (Utilities|Array|Add (LocalVariables|GetThetas) (* _total_whorls (* _whorls_percent_visible 0.01)))
  (for _index (range 1 (Math|Float|Truncate (* _total_whorls (* _whorls_percent_visible 0.01))))
    (Utilities|Array|Add (LocalVariables|GetThetas) (- (* _total_whorls (* _whorls_percent_visible 0.01)) (Math|Conversions|ToFloat(Integer) _index))))
  (return (LocalVariables|GetThetas)))